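; BP_FoodManager runs the eating phase, spawning food choices each round and feeding the selected one to the player.
; On start it creates the eating UI, finds the player and all BP_Food actors, reads the round count from the GameManager game instance and binds food interaction to selection.
; Each round re-randomizes every food's mesh and attribute.
; Eating or passing advances rounds; after the last, hunger depletes and the Kitchen level opens.
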(event `self.ReceiveBeginPlay`
  (`self.InitializeFoodManager`)
  (`self.SpawnFood`))

(event `BindEvents`
  (for _array_element (`self.FoodSpawns`)
    (add `/Game/Blueprints/Food/BP_Food.OnFoodInteraction` _array_element (delegate `SetSelectedFood`))))

(event `SetSelectedFood`
  (params (FoodItem :type "/Game/Blueprints/Food/BP_Food Object Reference"))
  (set `self.SelectedFood` FoodItem))

(event `FeedPlayer`
  (bind _selectedfood (`self.SelectedFood`))
  (`/Engine/EditorBlueprintResources/StandardMacros.IsValid` _selectedfood
    (:`Is Valid`
      (`/Game/Blueprints/Player/BP_Player.EatFood` (`self.Player`) _selectedfood)
      (`self.ProgressRound`))
    (:`Is Not Valid`
      (`KismetSystemLibrary.PrintString` "No valid selected food."))))

(event `PassRound`
  (`/Game/Blueprints/Player/BP_Player.PassRound` (`self.Player`))
  (`self.ProgressRound`))

(event `ProgressRound`
  (if (< (`self.CurrentRound`) (`self.RoundsCount`))
    (`/Engine/EditorBlueprintResources/StandardMacros.IncrementInt` (`self.CurrentRound`)
      (:`  `
        (`self.SpawnFood`)))
    (else
      (`self.ProgressDay`))))

(event `ProgressDay`
  (`PlayerChar.DepleteHunger` (`self.Player`) 20)
  (`Widget.RemoveFromParent` (`self.UI`))
  (`GameplayStatics.OpenLevel` "Kitchen"))

(fn `GetRandomAttribute`
  (returns (Attribute :type "/Game/Blueprints/Food/FoodAttribute Enum"))
  (return (`KismetArrayLibrary.Array_Random` (`self.Attributes`))))

(fn `GetRandomMesh`
  (returns (Mesh :type "StaticMesh Object Reference"))
  (return (`KismetArrayLibrary.Array_Random` (`self.FoodMeshes`))))

(fn `InitializeFoodManager`
  (bind _returnvalue (`|CreateWidget` "/Game/Blueprints/UI/UI_Eating.UI_Eating_C"))
  (bind _output_get (set `self.UI` _returnvalue))
  (`UserWidget.AddToViewport` _output_get 0)
  (bind _returnvalue_2 (`GameplayStatics.GetActorOfClass` "/Game/Blueprints/Player/BP_Player.BP_Player_C"))
  (set `self.Player` _returnvalue_2)
  (bind _outactors (`GameplayStatics.GetAllActorsOfClass` "/Game/Blueprints/Food/BP_Food.BP_Food_C"))
  (set `self.FoodSpawns` _outactors)
  (bind _asgame_manager (cast `GameManager` (`GameplayStatics.GetGameInstance`))
    (:`then`
      (bind _output_get_2 (set `self.GameManager` _asgame_manager))
      (bind _returnvalue_3 (`GameManager.GetRoundsCount` _output_get_2))
      (set `self.RoundsCount` _returnvalue_3))
    (:`CastFailed`
      (`KismetSystemLibrary.PrintString` "Casting to GM failed.")))
  (`self.BindEvents`))

(fn `SpawnFood`
  (for _array_element (`self.FoodSpawns`)
    (bind _mesh (`self.GetRandomMesh`))
    (`/Game/Blueprints/Food/BP_Food.SetMesh` _array_element _mesh)
    (bind _attribute (`self.GetRandomAttribute`))
    (`/Game/Blueprints/Food/BP_Food.SetAttribute` _array_element _attribute)))

(fn `UserConstructionScript`)