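; First-person player Blueprint with wandering movement, item pickup and hunger, health and condition effects from food and passing rounds.
; On BeginPlay it adds the wander input context, enabling movement and creating a reticle widget only in the GameManager's Wandering state.
; A forward camera line trace toggles the reticle over BPI_Interactable actors each tick and drives Interact, adding BP_Items to a five-slot inventory first.
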(event `self.ReceiveBeginPlay`
  (bind _asplayer_con (cast `PlayerCon` (`self.GetController`)))
  (`EnhancedInputSubsystemInterface.AddMappingContext` (pcsubsystem `EnhancedInputLocalPlayerSubsystem` _asplayer_con) "/Game/Blueprints/Player/Input/IMC_Wander.IMC_Wander" 0 (struct))
  (`KismetSystemLibrary.DelayUntilNextTick`)
  (if (`|EnumEquality` (`GameManager.CurrentState` (`self.gameManager`)) "Wandering")
    (bind _returnvalue (`|CreateWidget` "/Game/Blueprints/UI/UI_Reticle.UI_Reticle_C"))
    (`UserWidget.AddToViewport` _returnvalue 0)
    (set `self.CanMove` true)
    (else
      (set `self.CanMove` false))))

(event `self.ReceiveTick`
  (params (DeltaSeconds :type "Float (single-precision)"))
  (bind (_returnvalue _outhit) (`self.RaycastForward`))
  (bind (_bblockinghit _binitialoverlap _time _distance _location _impactpoint _normal _impactnormal _physmat _hitactor) (`GameplayStatics.BreakHitResult` _outhit))
  (`/Engine/EditorBlueprintResources/StandardMacros.IsValid` _hitactor
    (:`Is Valid`
      (cast `/Game/Blueprints/Core/BPI_Interactable` _hitactor
        (:`then`
          (`self.OnShowReticle`))
        (:`CastFailed`
          (`self.OnHideReticle`))))))

(event `EnhancedInput|/Game/Blueprints/Player/Input/Actions/IA_Move`
  (params (ActionValue :type "Vector2D Structure") (ElapsedSeconds :type "Float (double-precision)") (TriggeredSeconds :type "Float (double-precision)") (InputAction :type "InputAction Object Reference" :default "/Game/Blueprints/Player/Input/Actions/IA_Move.IA_Move"))
  (bind _movespeed (`self.MoveSpeed`))
  (:`Triggered`
    (if (`self.CanMove`)
      (`self.AddMovementInput` (`self.GetActorForwardVector`) (* ActionValue_Y _movespeed))
      (`self.AddMovementInput` (`self.GetActorRightVector`) (* ActionValue_X _movespeed)))))

(event `EnhancedInput|/Game/Blueprints/Player/Input/Actions/IA_MouseLook`
  (params (ActionValue :type "Vector2D Structure") (ElapsedSeconds :type "Float (double-precision)") (TriggeredSeconds :type "Float (double-precision)") (InputAction :type "InputAction Object Reference" :default "/Game/Blueprints/Player/Input/Actions/IA_MouseLook.IA_MouseLook"))
  (:`Triggered`
    (if (`self.CanMove`)
      (`self.AddControllerYawInput` ActionValue_X)
      (`self.AddControllerPitchInput` (* ActionValue_Y -1)))))

(event `EnhancedInput|/Game/Blueprints/Player/Input/Actions/IA_Interact`
  (params (ActionValue :type Boolean) (ElapsedSeconds :type "Float (double-precision)") (TriggeredSeconds :type "Float (double-precision)") (InputAction :type "InputAction Object Reference" :default "/Game/Blueprints/Player/Input/Actions/IA_Interact.IA_Interact"))
  (:`Started`
    (bind (_returnvalue _outhit) (`self.RaycastForward`))
    (bind (_bblockinghit _binitialoverlap _time _distance _location _impactpoint _normal _impactnormal _physmat _hitactor) (`GameplayStatics.BreakHitResult` _outhit))
    (if (`GameplayStatics.ObjectIsA` _hitactor "/Game/Blueprints/Items/BP_Item.BP_Item_C")
      (bind _asbp_item (cast `/Game/Blueprints/Items/BP_Item` _hitactor))
      (`self.AddItem` _asbp_item))
    (bind _asbpi_interactable (cast `/Game/Blueprints/Core/BPI_Interactable` _hitactor))
    (`/Game/Blueprints/Core/BPI_Interactable.Interact` _asbpi_interactable)))

(fn `AddItem`
  (params (Item :type "/Game/Blueprints/Items/BP_Item Object Reference"))
  (bind _items (`self.Items`))
  (if (< (`KismetArrayLibrary.Array_Length` _items) 5)
    (`KismetArrayLibrary.Array_Add` _items Item)))

(fn `EatFood`
  (params (FoodItem :type "/Game/Blueprints/Food/BP_Food Object Reference"))
  (switch `/Game/Blueprints/Food/FoodAttribute` (`/Game/Blueprints/Food/BP_Food.Attribute` FoodItem)
    (:`NewEnumerator0`
      (`self.RestoreHunger` 20))
    (:`NewEnumerator1`
      (`self.RestoreHunger` 40))
    (:`NewEnumerator2`
      (`self.RestoreHunger` 20)
      (`self.RestoreHealth` 20))
    (:`NewEnumerator3`
      (`self.RestoreHunger` 20)
      (set `self.Condition` "NewEnumerator1"))
    (:`NewEnumerator4`
      (`self.RestoreHunger` 20)
      (`self.DepleteHealth` 20))
    (:`NewEnumerator5`
      (`self.RestoreHunger` 20)
      (`self.DepleteHealth` 20))
    (:`NewEnumerator6`
      (`self.DepleteHunger` 40))
    (:`NewEnumerator7`
      (`self.RestoreHunger` 0)
      (set `self.Condition` "NewEnumerator2"))))

(fn `PassRound`
  (`self.DepleteHunger` 20))

(fn `UserConstructionScript`)