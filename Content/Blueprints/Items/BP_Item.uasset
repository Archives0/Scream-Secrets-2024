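; BP_Item is an interactable item that toggles between a spawned and despawned state without being destroyed.
; SpawnItem stores the given item type, sets the Spawned flag, shows the static mesh and enables its query and physics collision.
; Interact calls DespawnMesh, which clears the flag, hides the mesh and disables collision, leaving the actor available to spawn again.
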(event `/Game/Blueprints/Core/BPI_Interactable.Interact`
  (`self.DespawnMesh`))

(fn `DespawnMesh`
  (bind _staticmesh (`self.StaticMesh`))
  (set `self.Spawned` false)
  (`SceneComponent.SetVisibility` _staticmesh false false)
  (`PrimitiveComponent.SetCollisionEnabled` _staticmesh "NoCollision"))

(fn `SpawnItem`
  (params (Type :type "/Game/Blueprints/Items/ItemType Enum" :default "NewEnumerator0"))
  (bind _staticmesh (`self.StaticMesh`))
  (set `self.Spawned` true)
  (set `self.ItemType` Type)
  (`SceneComponent.SetVisibility` _staticmesh true false)
  (`PrimitiveComponent.SetCollisionEnabled` _staticmesh "QueryAndPhysics"))

(fn `UserConstructionScript`)